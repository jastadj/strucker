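; BP_TestPlayer is a test player character that moves along world X and Y from four directional input actions.
; Pressed and released events set per-direction values, which UpdateMovement sums into opposing axes every Tick, scales by MoveSpeed and passes to AddMovementInput.
; The construction script derives the flying braking deceleration from MoveSpeed, suggesting flying-style movement.
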(event Custom|UpdateMovement
  (bind _move_speed (Variables|Default|GetMove_Speed))
  ;[1 1 1] Movement Update
  (Pawn|Input|AddMovementInput (Math|Vector|MakeVector (* (+ (Variables|Default|GetMove_Left) (Variables|Default|GetMove_Right)) _move_speed) (* (+ (Variables|Default|GetMove_Up) (Variables|Default|GetMove_Down)) _move_speed) 0.0) 1.0 false))

(event EventBeginPlay)

(event Collision|EventActorBeginOverlap
  (params (OtherActor :type Actor%20Object%20Reference)))

(event EventTick
  (params (DeltaSeconds :type Float%20%28single-precision%29))
  (CallFunction|UpdateMovement))

(event Input|ActionEvents|InputActionMoveLeft
  (params (Key :type Key%20Structure))
  ;[1 1 1] Movement Direction
  (:Pressed
    (Variables|Default|SetMove_Left 1.0))
  (:Released
    (Variables|Default|SetMove_Left 0.0)))

(event Input|ActionEvents|InputActionMoveRight
  (params (Key :type Key%20Structure))
  ;[1 1 1] Movement Direction
  (:Pressed
    (Variables|Default|SetMove_Right -1.0))
  (:Released
    (Variables|Default|SetMove_Right 0.0)))

(event Input|ActionEvents|InputActionMoveUp
  (params (Key :type Key%20Structure))
  ;[1 1 1] Movement Direction
  (:Pressed
    (Variables|Default|SetMove_Up 1.0))
  (:Released
    (Variables|Default|SetMove_Up 0.0)))

(event Input|ActionEvents|InputActionMoveDown
  (params (Key :type Key%20Structure))
  ;[1 1 1] Movement Direction
  (:Pressed
    (Variables|Default|SetMove_Down -1.0))
  (:Released
    (Variables|Default|SetMove_Down 0.0)))

(fn ConstructionScript
  (Variables|/Script/Engine.CharacterMovementComponent|SetBrakingDecelerationFlying (Variables|Character|GetCharacterMovement) (* (Variables|Default|GetMove_Speed) 1.5)))