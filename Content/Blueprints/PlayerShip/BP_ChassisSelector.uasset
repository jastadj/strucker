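; BP_ChassisSelector picks the player ship's chassis model from saved player data when play begins.
; On BeginPlay it casts the game instance to GameInstance_Player and switches on the ShipChassis enum in PlayerData.
; Each case stores its corresponding model in ChassisModel and prints the object name for debugging.
; The graph only sets that variable, and a failed cast just prints an error.
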(event EventBeginPlay
  (bind _asgame_instance_player (Utilities|Casting|CastToGameInstance_Player (Game|GetGameInstance))
    (:then
      (switch Utilities|FlowControl|Switch|SwitchonENUM_ChassisTypes (Utilities|Struct|BreakStruct_PlayerData (Variables|/Game/Blueprints/Player/GameInstance_Player.GameInstance_Player_C|GetPlayerData _asgame_instance_player))
        (:NewEnumerator1
          (bind _output_get (Variables|Default|SetChassisModel "/Game/Models/TestShip/testchassis1.testchassis1"))
          (Development|PrintString (Utilities|String|Append "selected model " (Utilities|GetObjectName _output_get))))
        (:NewEnumerator2
          (bind _output_get_2 (Variables|Default|SetChassisModel "/Game/Models/spacetruck/spacetruck_1.spacetruck_1"))
          (Development|PrintString (Utilities|String|Append "selected model " (Utilities|GetObjectName _output_get_2))))
        (:NewEnumerator3
          (bind _output_get_3 (Variables|Default|SetChassisModel "/Game/Models/TestShip/testship.testship"))
          (Development|PrintString (Utilities|String|Append "selected model " (Utilities|GetObjectName _output_get_3))))))
    (:CastFailed
      (Development|PrintString "Error casting game instance"))))

(event EventTick
  (params (DeltaSeconds :type Float%20%28single-precision%29)))